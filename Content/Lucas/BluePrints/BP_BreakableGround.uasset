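; BP_BreakableGround is a floor that shatters and drops out from under the player when they step on it.
; Player overlap disables the trigger, makes the Geometry Collection floor ignore the Pawn channel and the player capsule's movement, and plays a camera shake.
; It releases the pieces with a wide kinematic field and cluster crumbling, then reapplies the field after a brief delay.
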(event EventBeginPlay)

(event Collision|EventActorBeginOverlap
  (params (OtherActor :type Actor%20Object%20Reference))
  (bind _returnvalue (Transformation|GetActorLocation))
  (bind _gc_floor (Variables|Default|GetGC_Floor))
  (if (== OtherActor (Game|Player|GetPlayerPawn 0))
    (Collision|SetCollisionEnabled (Variables|Default|GetBreakTrigger) "NoCollision")
    (Collision|SetCollisionResponsetoChannel _gc_floor "ECC_Pawn" "ECR_Ignore")
    (Class|PrimitiveComponent|IgnoreComponentwhenMoving (Actor|GetComponentbyClass OtherActor "/Script/Engine.CapsuleComponent") _gc_floor true)
    (CameraShakes|StartCameraShake (Game|GetPlayerCameraManager 0) "/Game/Lucas/BluePrints/BP_LegacyCameraShake.BP_LegacyCameraShake_C" 1.0 "CameraLocal" "0, 0, 0")
    (Class|GeometryCollectionComponent|ApplyKinematicField _gc_floor 1e+05 _returnvalue)
    (Class|GeometryCollectionComponent|CrumbleActiveClusters _gc_floor)
    (Utilities|FlowControl|Delay 0.1)
    (Class|GeometryCollectionComponent|ApplyKinematicField _gc_floor 1e+05 _returnvalue)))

(event EventTick
  (params (DeltaSeconds :type Float%20%28single-precision%29)))

(fn ConstructionScript)