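; BP_Wall is a destructible Geometry Collection wall that reacts to being hit by a BP_RollingStone or BP_DemolitionBall.
; The first qualifying hit fires the EStateChanged dispatcher with Break and adds an impulse built from the inverted hit normal impulse plus a large fixed offset.
; Its own handler, bound on BeginPlay, stores the state, plays a 2D rock-break sound and runs two camera shakes separated by a delay.
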(event OnComponentHit(GeometryCollection)
  (params (HitComponent :type Primitive%20Component%20Object%20Reference) (OtherActor :type Actor%20Object%20Reference) (OtherComp :type Primitive%20Component%20Object%20Reference) (NormalImpulse :type Vector :default "0, 0, 0") (Hit :type Hit%20Result%20Structure%20%28by%20ref%29))
  (Utilities|Casting|CastToBP_RollingStone OtherActor
    (:then
      _)
    (:CastFailed
      (Utilities|Casting|CastToBP_DemolitionBall OtherActor)))
  (Utilities|FlowControl|DoOnce false
    (:Completed
      (Default|CallEStateChanged "NewEnumerator1")
      (Physics|AddImpulse (Variables|Default|GetGeometryCollection) (+ (* NormalImpulse -1.0) "100000.000000,10000.000000,100000.000000") "None" false)
      (Utilities|FlowControl|Delay 1.0))))

(event Custom|E_StateChanged_Event
  (params (State :type E_Wall%20Enum :default "NewEnumerator0"))
  (bind _output_get (Variables|Default|SetState State))
  (switch Utilities|FlowControl|Switch|SwitchonE_Wall _output_get
    (:NewEnumerator1
      (Audio|PlaySound2D "/Game/System/RollingStone/s_breakrock.s_breakrock" 1.0 1.0 0.4 0 0)
      (Class|LegacyCameraShake|StartLegacyCameraShake (Game|GetPlayerCameraManager 0) "/Game/System/DectructibleWall/CS_Destruction.CS_Destruction_C" 1.0 "CameraLocal" "0, 0, 0")
      (Utilities|FlowControl|Delay 1.5)
      (Class|LegacyCameraShake|StartLegacyCameraShake (Game|GetPlayerCameraManager 0) "/Game/System/DectructibleWall/CS_DestructionCluster.CS_DestructionCluster_C" 1.0 "CameraLocal" "0, 0, 0"))))

(event EventBeginPlay
  (EventDispatchers|AssignEStateChanged (delegate Custom|E_StateChanged_Event)))

(fn ConstructionScript)