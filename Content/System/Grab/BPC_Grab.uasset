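; BPC_Grab is a component that lets the third-person character pick up and carry physics-simulating interact actors.
; It grabs the interact component's current object with the character's PhysicsHandle at a set range along the follow camera's view.
; A looping timer, rather than Tick, keeps moving the handle target to that point with zero rotation.
; Completing IA_Grab releases the mesh and clears the timer; StartGrab has no caller here.
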(event Input|EnhancedActionEvents|EnhancedInputActionIA_Grab
  (params (ActionValue :type Boolean) (ElapsedSeconds :type Float%20%28double-precision%29) (TriggeredSeconds :type Float%20%28double-precision%29) (InputAction :type Input%20Action%20Object%20Reference :default "/Game/Input/Actions/IA_Grab.IA_Grab"))
  (:Completed
    (if (and (Variables|Default|GetIsGrab?) (Utilities|IsValid (Variables|Default|GetCurrent%20grabbed%20Mesh)))
      (CallFunction|StopGrab))))

(event EventBeginPlay
  (bind _asbp_third_person_character (Utilities|Casting|CastToBP_ThirdPersonCharacter (Components|GetOwner)))
  (bind _output_get (Variables|Default|SetPlayer%20ref _asbp_third_person_character))
  (Variables|Default|SetPhysics%20Handle (Variables|/Game/ThirdPerson/Blueprints/BP_ThirdPersonCharacter.BP_ThirdPersonCharacter_C|GetPhysicsHandle _output_get))
  (Variables|Default|SetBPC%20Interact (Variables|/Game/ThirdPerson/Blueprints/BP_ThirdPersonCharacter.BP_ThirdPersonCharacter_C|GetBPC_Interact (Variables|Default|GetPlayer%20ref))))

(fn GrabObject
  (bind _player_ref (Variables|Default|GetPlayer%20ref))
  (bind _followcamera (Variables|/Game/ThirdPerson/Blueprints/BP_ThirdPersonCharacter.BP_ThirdPersonCharacter_C|GetFollowCamera _player_ref))
  (bind _asbp_interact_actor (Utilities|Casting|CastToBP_InteractActor (Variables|/Game/System/Interact/BPC_Interact.BPC_Interact_C|GetCurrent%20Object (Variables|Default|GetBPC%20Interact))))
  (if (Physics|IsSimulatingPhysics (Variables|/Game/System/Interact/BP_InteractActor.BP_InteractActor_C|GetStaticMesh _asbp_interact_actor) "None")
    (Variables|Default|SetIsGrab? true)
    (Variables|Default|SetCurrent%20grabbed%20Mesh (Variables|/Game/System/Interact/BP_InteractActor.BP_InteractActor_C|GetStaticMesh _asbp_interact_actor))
    (Physics|Components|PhysicsHandle|GrabComponentatLocationwithRotation (Variables|Default|GetPhysics%20Handle) (Variables|/Game/System/Interact/BP_InteractActor.BP_InteractActor_C|GetStaticMesh _asbp_interact_actor) "None" (+ (Transformation|GetWorldLocation _followcamera) (* (Math|Vector|GetForwardVector _followcamera) (Variables|Default|GetRange))) "0, 0, 0")))

(fn SetGrabbedObjectLocation
  (bind _player_ref (Variables|Default|GetPlayer%20ref))
  (bind _followcamera (Variables|/Game/ThirdPerson/Blueprints/BP_ThirdPersonCharacter.BP_ThirdPersonCharacter_C|GetFollowCamera _player_ref))
  (Utilities|IsValid (Variables|Default|GetBPC%20Interact)
    (:Is%20Valid
      (Class|PhysicsHandleComponent|SetTargetLocationandRotation (Variables|Default|GetPhysics%20Handle) (+ (Transformation|GetWorldLocation _followcamera) (* (Math|Vector|GetForwardVector _followcamera) (Variables|Default|GetRange))) "0, 0, 0"))))

(fn StartGrab
  (CallFunction|GrabObject)
  (bind _returnvalue (Utilities|Time|SetTimerbyFunctionName 0 "Set Grabbed Object Location" 0.05 true))
  (Variables|Default|SetHandle%20Grab _returnvalue))

(fn StopGrab
  (Physics|Components|PhysicsHandle|ReleaseComponent (Variables|Default|GetPhysics%20Handle))
  (Variables|Default|SetIsGrab? false)
  (Utilities|Time|ClearandInvalidateTimerbyHandle (Variables|Default|GetHandle%20Grab))
  (Variables|Default|SetCurrent%20grabbed%20Mesh 0))