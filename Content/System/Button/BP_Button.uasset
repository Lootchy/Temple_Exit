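; BP_Button is a button actor that becomes pressed when a BP_LaunchBall overlaps its sphere trigger.
; The overlap fires the EButtonPressed event dispatcher with a Pressed state, after an exact class check on the overlapping actor.
; The button binds to its own dispatcher on BeginPlay to store the state and print a debug message.
; The construction script applies a configurable material to Cylinder1.
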(event OnComponentBeginOverlap(Sphere)
  (params (OverlappedComponent :type Primitive%20Component%20Object%20Reference) (OtherActor :type Actor%20Object%20Reference) (OtherComp :type Primitive%20Component%20Object%20Reference) (OtherBodyIndex :type Integer) (bFromSweep :type Boolean) (SweepResult :type Hit%20Result%20Structure%20%28by%20ref%29))
  (if (== (Utilities|GetClass OtherActor) "/Game/System/Button/BP_LaunchBall.BP_LaunchBall_C")
    (Default|CallEButtonPressed "NewEnumerator1")))

(event Custom|E_ButtonPressed_Event
  (params (State :type E_ButtonState%20Enum :default "NewEnumerator0"))
  (bind _output_get (Variables|Default|SetState State))
  (switch Utilities|FlowControl|Switch|SwitchonE_ButtonState _output_get
    (:NewEnumerator1
      (Development|PrintString "button pressed"))))

(event EventBeginPlay
  (EventDispatchers|AssignEButtonPressed (delegate Custom|E_ButtonPressed_Event)))

(fn ConstructionScript
  (Rendering|Material|SetMaterial (Variables|Default|GetCylinder1) 0 (Variables|Default|GetMaterial)))