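; BP_LaunchBall is an interactable ball the player grabs through BPCGrab and throws with a charged launch.
; Holding IA_UseItem scales horizontal and upward force by hold time within clamps, while a looping timer predicts and debug-draws the arc.
; That update also builds the launch vector from camera direction, remapping pitch for lift.
; Releasing or canceling stops prediction, resets the forces, drops the ball and applies the stored vector as a velocity-change impulse.
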(event Custom|Update%20Projectiel%20PAth
  (bind _returnvalue (Game|GetPlayerCameraManager 0))
  (bind _force (Variables|Default|GetForce))
  (bind _up_force (Variables|Default|GetUp%20Force))
  (bind _returnvalue_2 (Camera|GetCameraRotation _returnvalue))
  (bind _returnvalue_3 (Math|Vector|GetForwardVector _returnvalue_2))
  (bind _z (Math|Vector|BreakVector _returnvalue_3))
  (bind _returnvalue_4 (* _returnvalue_3 _force))
  (bind (_x _y) (Math|Vector|BreakVector _returnvalue_4))
  (bind _returnvalue_5 (Math|Float|MapRangeUnclamped _z 0.0 1.0 3.0 1e+01))
  (bind _returnvalue_6 (* _returnvalue_5 _up_force))
  (Class|GameplayStatics|BlueprintPredictProjectilePathAdvanced (Utilities|Struct|MakePredictProjectilePathParams (Transformation|GetWorldLocation (Variables|Default|GetStaticMesh)) (Math|Vector|MakeVector _x _y _returnvalue_6) true 0.0 1.0 true "ECC_WorldStatic" "ObjectTypeQuery1" (Utilities|Array|MakeArray self) 2e+01 0.0 "ForDuration" 1.0 false))
  (Variables|Default|SetForce%20vector (Math|Vector|MakeVector _x _y _returnvalue_6)))

(event Custom|Draw%20Projectile%20Path
  (bind _returnvalue (Utilities|Time|SetTimerbyEvent (delegate Custom|Update%20Projectiel%20PAth) 0.1 true))
  (Variables|Default|SetHandle%20Prediction _returnvalue))

(event Custom|Stop%20Prediction
  (Utilities|Time|ClearandInvalidateTimerbyHandle (Variables|Default|GetHandle%20Prediction)))

(event Input|EnhancedActionEvents|EnhancedInputActionIA_UseItem
  (params (ActionValue :type Boolean) (ElapsedSeconds :type Float%20%28double-precision%29) (TriggeredSeconds :type Float%20%28double-precision%29) (InputAction :type Input%20Action%20Object%20Reference :default "/Game/Input/Actions/IA_UseItem.IA_UseItem"))
  (bind _force_vector (Variables|Default|GetForce%20vector))
  (:Triggered
    (Variables|Default|SetForce (Math|Float|Clamp(Float) (* (Variables|Default|GetForce) ElapsedSeconds) 1e+03 6e+03))
    (Variables|Default|SetUp%20Force (Math|Float|Clamp(Float) (* ElapsedSeconds (Variables|Default|GetUp%20Force)) 1.5e+02 5e+02)))
  (:Started
    (bind _player_ref (Variables|Default|GetPlayer%20Ref)
      (:then
        (if (== (Variables|/Game/System/Grab/BPC_Grab.BPC_Grab_C|GetCurrent%20grabbed%20Mesh (Variables|/Game/ThirdPerson/Blueprints/BP_ThirdPersonCharacter.BP_ThirdPersonCharacter_C|GetBPC_Grab _player_ref)) (Variables|Default|GetStaticMesh))
          (CallFunction|DrawProjectilePath)))
      (:else)))
  (:Canceled
    (bind _player_ref_2 (Variables|Default|GetPlayer%20Ref :!label _label)
      (:then
        (if (== (Variables|/Game/System/Grab/BPC_Grab.BPC_Grab_C|GetCurrent%20grabbed%20Mesh (Variables|/Game/ThirdPerson/Blueprints/BP_ThirdPersonCharacter.BP_ThirdPersonCharacter_C|GetBPC_Grab _player_ref_2)) (Variables|Default|GetStaticMesh))
          (CallFunction|StopPrediction)
          (Variables|Default|SetForce 5e+02)
          (Variables|Default|SetUp%20Force 1.5e+02)
          (Default|StopGrab (Variables|/Game/ThirdPerson/Blueprints/BP_ThirdPersonCharacter.BP_ThirdPersonCharacter_C|GetBPC_Grab (Variables|Default|GetPlayer%20Ref)))
          (Physics|AddImpulse (Variables|Default|GetStaticMesh) _force_vector "None" true)
          (Development|PrintString (Utilities|String|ToString(Vector) _force_vector))))
      (:else)))
  (:Completed
    (goto _label)))

(event EventBeginPlay
  (|CallParentFunction)
  (Input|EnableInput (Game|GetPlayerController 0)))

(event EventInteract
  (params (Player%20ref :type BP%20Third%20Person%20Character%20Object%20Reference))
  (Variables|Default|SetPlayer%20Ref Player%20ref)
  (|CallParentFunction Player%20ref)
  (Default|StartGrab (Variables|/Game/ThirdPerson/Blueprints/BP_ThirdPersonCharacter.BP_ThirdPersonCharacter_C|GetBPC_Grab Player%20ref)))

(fn ConstructionScript
  (|CallParentFunction))