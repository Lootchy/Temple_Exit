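; Player interaction component for BP_ThirdPersonCharacter that highlights and activates the object the follow camera looks at.
; A fast looping timer runs Raycast Interact, a debug-drawn Visibility trace that tracks the hit actor and toggles its outline through messages.
; On IA_Interact completion, it sends InteractMessage to the tracked actor and plays a sound.
; Raycast Outline is a near-duplicate without debug drawing or target clearing, not called here.
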(event Input|EnhancedActionEvents|EnhancedInputActionIA_Interact
  (params (ActionValue :type Boolean) (ElapsedSeconds :type Float%20%28double-precision%29) (TriggeredSeconds :type Float%20%28double-precision%29) (InputAction :type Input%20Action%20Object%20Reference :default "/Game/Input/Actions/IA_Interact.IA_Interact"))
  (:Completed
    (bind _current_object (Variables|Default|GetCurrent%20Object)
      (:then
        (Class|BPIInteract|Interact(Message) _current_object (Variables|Default|GetPlayer%20ref))
        (Audio|PlaySound2D 0 1.0 1.0 0.0 0 0))
      (:else))))

(event EventBeginPlay
  (bind _asbp_third_person_character (Utilities|Casting|CastToBP_ThirdPersonCharacter (Components|GetOwner)))
  (Variables|Default|SetPlayer%20ref _asbp_third_person_character)
  (bind _returnvalue (Utilities|Time|SetTimerbyFunctionName 0 "Raycast Interact" 0.05 true))
  (Variables|Default|SetHandle%20Raycast _returnvalue))

(fn RaycastInteract
  (bind _player_ref (Variables|Default|GetPlayer%20ref))
  (bind _followcamera (Variables|/Game/ThirdPerson/Blueprints/BP_ThirdPersonCharacter.BP_ThirdPersonCharacter_C|GetFollowCamera _player_ref))
  (bind _returnvalue (Transformation|GetWorldLocation _followcamera))
  (bind (_outhit _returnvalue_2) (Collision|LineTraceByChannel _returnvalue (+ _returnvalue (* (Math|Vector|GetForwardVector _followcamera) (Variables|Default|GetRange))) "TraceTypeQuery1" false 0 "ForDuration"))
  (if _returnvalue_2
    (if (!= (Variables|Default|GetCurrent%20Object) (.HitActor (Collision|BreakHitResult _outhit)))
      (Class|BPIInteract|ShowOutline(Message) (Variables|Default|GetCurrent%20Object) false)
      (bind _output_get (Variables|Default|SetCurrent%20Object (.HitActor (Collision|BreakHitResult _outhit))))
      (Class|BPIInteract|ShowOutline(Message) _output_get true))
    (else
      (Class|BPIInteract|ShowOutline(Message) (Variables|Default|GetCurrent%20Object) false)
      (Variables|Default|SetCurrent%20Object 0))))

(fn RaycastOutline
  (bind _player_ref (Variables|Default|GetPlayer%20ref))
  (bind _followcamera (Variables|/Game/ThirdPerson/Blueprints/BP_ThirdPersonCharacter.BP_ThirdPersonCharacter_C|GetFollowCamera _player_ref))
  (bind _returnvalue (Transformation|GetWorldLocation _followcamera))
  (bind (_outhit _returnvalue_2) (Collision|LineTraceByChannel _returnvalue (+ _returnvalue (* (Math|Vector|GetForwardVector _followcamera) (Variables|Default|GetRange))) "TraceTypeQuery1" false 0 "None"))
  (if _returnvalue_2
    (if (!= (Variables|Default|GetCurrent%20Object) (.HitActor (Collision|BreakHitResult _outhit)))
      (Class|BPIInteract|ShowOutline(Message) (Variables|Default|GetCurrent%20Object) false)
      (bind _output_get (Variables|Default|SetCurrent%20Object (.HitActor (Collision|BreakHitResult _outhit))))
      (Class|BPIInteract|ShowOutline(Message) _output_get true))
    (else
      (Class|BPIInteract|ShowOutline(Message) (Variables|Default|GetCurrent%20Object) false))))